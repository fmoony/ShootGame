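; BP_BakedEightPreview is an experiment helper actor for previewing a baked eight-way crouch stance on the player's ShooterStancePreviewPawn.
; On its first valid tick it sets tick prerequisites so it ticks after the pawn and the pawn's skeletal mesh component ticks after it.
; It also prints an on-screen controls hint once, and does no other work in the graph shown.
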(event `self.ReceiveTick`
  (params (DeltaSeconds :type "Float (single-precision)"))
  (bind _asshooter_stance_preview_pawn (cast `ShooterStancePreviewPawn` (`GameplayStatics.GetPlayerPawn` 0)))
  (bind _asskeletal_mesh_component (cast `SkeletalMeshComponent` (`self.GetComponentByClass` _asshooter_stance_preview_pawn "/Script/Engine.SkeletalMeshComponent")))
  (if (not (`self.bInitialized`))
    (`self.AddTickPrerequisiteActor` _asshooter_stance_preview_pawn)
    (`ActorComponent.AddTickPrerequisiteActor` _asskeletal_mesh_component self)
    (set `self.bInitialized` true)
    (`KismetSystemLibrary.PrintString` "BAKED EIGHT CROUCH | WASD Move | Release Stop | Mouse Look | V View | T Pause" true true (struct :`G` 0.66 :`B` 1.0 :`A` 1.0) 9999.0 "OWLOCAL")))

(fn `UserConstructionScript`)